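; Base brick actor that loses HP when batted, showing crack decals until it shatters, and slides away in the batted direction.
; Timelines move it in 100-unit grid steps, with box traces checking for blockers and line traces for support; unsupported bricks fall step by step.
; Meeting a player on a bat or below triggers HarmPlayer, which destroys the brick and always box-traces along MoveDirection for damage, even after falls.
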(event `OnBatted`
  (bind _hp (`self.HP`))
  (bind _output (`|GetArrayItem` (`self.Cracks`) (- _hp 1)))
  (bind _result (`/Engine/EditorBlueprintResources/StandardMacros.DecrementInt` _hp)
    (:`  `
      (set `self.HP` _result)
      (`KismetSystemLibrary.PrintString` (`KismetStringLibrary.Conv_IntToString` _hp))
      (if (<= _hp 0)
        (`GameplayStatics.PlaySoundAtLocation` "/Game/sOUND/rockShatter.rockShatter" (`self.K2_GetActorLocation`) (struct) 1.0 1.2 0.0 null null null null)
        (`self.K2_DestroyActor`)
        (else
          (`GameplayStatics.PlaySoundAtLocation` "/Game/sOUND/batBrickCue.batBrickCue" (`self.K2_GetActorLocation`) (struct) 0.7 1.0 0.0 null null null null)
          (`DecalComponent.SetDecalMaterial` (`self.SideDecal`) _output)
          (`DecalComponent.SetDecalMaterial` (`self.TopDecal1`) _output)
          (`DecalComponent.SetDecalMaterial` (`self.SideDecal1`) _output)
          (`DecalComponent.SetDecalMaterial` (`self.SideDecal2`) _output)
          (`DecalComponent.SetDecalMaterial` (`self.SideDecal3`) _output))))))

(event `self.ReceiveBeginPlay`
  (`TimelineComponent.SetPlayRate` (`self.FallTimeline`) 2.0)
  (`TimelineComponent.SetPlayRate` (`self.MoveTimeline`) 2.0)
  (bind (_outhit _returnvalue) (`self.FoundSomethingBelow`))
  (if (not _returnvalue)
    (`self.Fall`)))

(event `Bat`
  (params (Direction :type "/Game/Blueprints/E_MoveDirections Enum" :default "NewEnumerator0"))
  (`self.OnBatted`)
  (bind (_outhit _true) (`self.IsBlocked` Direction))
  (cast `/Game/Blueprints/Character/BP_Player` (`.HitActor` (`GameplayStatics.BreakHitResult` _outhit))
    (:`then`
      (`self.HarmPlayer` false))
    (:`CastFailed`
      (if (not _true)
        (`self.TryMove` Direction)))))

(event `TryMove`
  (params (Direction :type "/Game/Blueprints/E_MoveDirections Enum" :default "NewEnumerator0"))
  (bind (_movedirection_x _movedirection_y) (`KismetMathLibrary.BreakVector2D` (`self.MoveDirection`)))
  (bind (_locationatmovestart_x _locationatmovestart_y _locationatmovestart_z) (`KismetMathLibrary.BreakVector` (`self.LocationAtMoveStart`)))
  (if (not (`self.isMoving`))
    (set `self.isMoving` true)
    (set `self.LocationAtMoveStart` (`self.K2_GetActorLocation`))
    (switch `/Game/Blueprints/E_MoveDirections` Direction
      (:`NewEnumerator0`
        (set `self.MoveDirection` (1.0 0.0))
        (bind (_direction _normalizedtime) (`Timeline|MoveTimeline` :!via `PlayFromStart` :!label _label)
          (:`Update`
            (`self.K2_SetActorLocation` (`KismetMathLibrary.MakeVector` (+ (* _movedirection_x 100.0 _normalizedtime) _locationatmovestart_x) (+ (* _movedirection_y 100.0 _normalizedtime) _locationatmovestart_y) _locationatmovestart_z) false true))
          (:`Finished`
            (set `self.isMoving` false)
            (`self.FindNextMove` Direction))))
      (:`NewEnumerator1`
        (set `self.MoveDirection` (-1.0 0.0))
        (goto _label :!via `PlayFromStart`))
      (:`NewEnumerator2`
        (set `self.MoveDirection` (0.0 1.0))
        (goto _label :!via `PlayFromStart`))
      (:`NewEnumerator3`
        (set `self.MoveDirection` (0.0 -1.0))
        (goto _label :!via `PlayFromStart`)))))

(event `HarmPlayer`
  (params (isFalling :type Boolean))
  (bind _returnvalue (`self.K2_GetActorLocation`))
  (bind (_returnvalue_x _returnvalue_y _returnvalue_z) (`KismetMathLibrary.BreakVector` (`KismetMathLibrary.Vector_Down`)))
  (bind _returnvalue_2 (`self.K2_GetActorLocation`))
  (bind (_movedirection_x _movedirection_y) (`KismetMathLibrary.BreakVector2D` (`self.MoveDirection`)))
  (if isFalling
    (bind _outhits (`KismetSystemLibrary.BoxTraceMulti` :`Start` _returnvalue :`End` (+ _returnvalue (`KismetMathLibrary.MakeVector` 0.0 0.0 (* _returnvalue_z 100.0))) :`HalfSize` (49.0 49.0 49.0) :`TraceChannel` "TraceTypeQuery1" :`DrawDebugType` "ForDuration"))
    (set `self.Collisions` _outhits)
    (else
      (bind _outhits_2 (`KismetSystemLibrary.BoxTraceMulti` :`Start` _returnvalue_2 :`End` (+ _returnvalue_2 (`KismetMathLibrary.MakeVector` (* _movedirection_x 100.0) (* _movedirection_y 100.0))) :`HalfSize` (49.0 49.0 49.0) :`TraceChannel` "TraceTypeQuery1" :`DrawDebugType` "ForDuration"))
      (set `self.Collisions` _outhits_2)))
  (for _array_element (`self.Collisions`)
    (bind _asbp_player (cast `/Game/Blueprints/Character/BP_Player` (`.HitActor` (`GameplayStatics.BreakHitResult` _array_element))))
    (`/Game/Blueprints/damageSystem/BPC_DamageSystem.TakeDamage` (`/Game/Blueprints/Character/BP_Player.BPC_DamageSystem` _asbp_player) (make `/Game/Blueprints/damageSystem/S_DamageInfo` 1.0 "NewEnumerator1")))
  (`self.K2_DestroyActor`))

(event `FindNextMove`
  (params (Direction :type "/Game/Blueprints/E_MoveDirections Enum" :default "NewEnumerator0"))
  (bind (_returnvalue_x _returnvalue_y _returnvalue_z) (`KismetMathLibrary.BreakVector` (`self.K2_GetActorLocation`)))
  (bind (_locationatfallstart_x _locationatfallstart_y _locationatfallstart_z) (`KismetMathLibrary.BreakVector` (`self.LocationAtFallStart`)))
  (bind (_outhit _returnvalue) (`self.FoundSomethingBelow`))
  (if _returnvalue
    (cast `/Game/Blueprints/Character/BP_Player` (`.HitActor` (`GameplayStatics.BreakHitResult` _outhit))
      (:`then`
        (`self.HarmPlayer` false))
      (:`CastFailed`
        (bind (_outhit_2 _true) (`self.IsBlocked` Direction))
        (if (not _true)
          (`self.TryMove` Direction))))
    (else
      (set `self.LocationAtFallStart` (`self.K2_GetActorLocation`) :!label _label_2)
      (bind (_direction _normalizedtime) (`Timeline|FallTimeline` :!via `PlayFromStart`)
        (:`Update`
          (`self.K2_SetActorLocation` (`KismetMathLibrary.MakeVector` _locationatfallstart_x _locationatfallstart_y (+ _locationatfallstart_z (* _normalizedtime -100.0))) false true))
        (:`Finished`
          (bind (_outhit_3 _returnvalue_2) (`self.FoundSomethingBelow`))
          (if _returnvalue_2
            (cast `/Game/Blueprints/Character/BP_Player` (`.HitActor` (`GameplayStatics.BreakHitResult` _outhit_3))
              (:`then`
                (`self.HarmPlayer` false))
              (:`CastFailed`
                (`/Engine/EditorBlueprintResources/StandardMacros.DoOnce` false
                  (:`Completed`
                    (`GameplayStatics.PlaySoundAtLocation` "/Game/sOUND/brickLand.brickLand" (`KismetMathLibrary.MakeVector` _returnvalue_x _returnvalue_y (+ _returnvalue_z -50.0)) (struct) 0.5 1.0 0.0 null null null null)))))
            (else
              (`self.Fall`))))))))

(event `Fall`
  (goto _label_2))

(fn `FoundSomethingBelow`
  (returns (OutHit :type "HitResult Structure") (ReturnValue :type Boolean))
  (bind _returnvalue (`self.K2_GetActorLocation`))
  (bind (_outhit _returnvalue_2) (`KismetSystemLibrary.LineTraceSingle` :`Start` _returnvalue :`End` (+ _returnvalue (* 60.0 (`KismetMathLibrary.Vector_Down`))) :`TraceChannel` "TraceTypeQuery1" :`DrawDebugType` "ForDuration"))
  (return _outhit _returnvalue_2))

(fn `IsBlocked`
  (params (DirectionToCheck :type "/Game/Blueprints/E_MoveDirections Enum" :default "NewEnumerator0"))
  (returns (OutHit :type "HitResult Structure") (True :type Boolean))
  (locals (CheckDirection :type "Vector2D Structure"))
  (bind _returnvalue (`self.K2_GetActorLocation`))
  (bind (_checkdirection_x _checkdirection_y) (`KismetMathLibrary.BreakVector2D` (`local.CheckDirection`)))
  (switch `/Game/Blueprints/E_MoveDirections` DirectionToCheck
    (:`NewEnumerator0`
      (set `local.CheckDirection` (1.0 0.0)))
    (:`NewEnumerator1`
      (set `local.CheckDirection` (-1.0 0.0)))
    (:`NewEnumerator2`
      (set `local.CheckDirection` (0.0 1.0)))
    (:`NewEnumerator3`
      (set `local.CheckDirection` (0.0 -1.0))))
  (bind (_outhit _returnvalue_2) (`KismetSystemLibrary.BoxTraceSingle` :`Start` _returnvalue :`End` (+ _returnvalue (`KismetMathLibrary.MakeVector` (* _checkdirection_x 100.0) (* _checkdirection_y 100.0))) :`HalfSize` (49.0 49.0 49.0) :`TraceChannel` "TraceTypeQuery3" :`DrawDebugType` "ForDuration"))
  (return _outhit _returnvalue_2))

(fn `UserConstructionScript`)
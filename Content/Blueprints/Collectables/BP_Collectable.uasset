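; BP_Collectable is a power-up pickup that grants its PowerType to the player on touch.
; On BeginPlay it picks a gem mesh by type, with Jump and Health sharing CoffinGem while a HeartGem assignment is left unconnected.
; The Animate timeline ping-pongs through a FlipFlop, bobbing and rotating the mesh around its starting transform.
; Sphere overlap with BP_Player plays a bite sound, calls GetPowerUp and destroys the actor.
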(event `self.ReceiveBeginPlay`
  (bind _hometransform (`self.HomeTransform`))
  (bind _staticmesh (`self.StaticMesh`))
  (`|ExecutionSequence`
    (:`then_0`
      (switch `/Game/Blueprints/Collectables/E_PowerupTypes` (`self.PowerType`)
        (:`NewEnumerator0`
          (`StaticMeshComponent.SetStaticMesh` _staticmesh "/Game/Textures/Collectables/CoffinGem.CoffinGem" :!label _label))
        (:`NewEnumerator1`
          (goto _label))
        (:`NewEnumerator2`
          (`StaticMeshComponent.SetStaticMesh` _staticmesh "/Game/Textures/Collectables/PointyGem.PointyGem"))
        (:`NewEnumerator3`
          (`StaticMeshComponent.SetStaticMesh` _staticmesh "/Game/Textures/Collectables/HexagonGem.HexagonGem"))))
    (:`then_1`
      (set `self.HomeTransform` (`self.GetTransform`))
      (bind (_direction _normalizedtime) (`Timeline|Animate` :!via `PlayFromStart` :!label _label_2)
        (:`Update`
          (`SceneComponent.K2_SetWorldLocationAndRotation` (`self.StaticMesh`) (`KismetMathLibrary.MakeVector` (.x (.location _hometransform)) (.y (.location _hometransform)) (+ (* _normalizedtime 40.0) (.z (.location _hometransform)))) (`KismetMathLibrary.MakeRotator` (.roll (.rotation _hometransform)) (.pitch (.rotation _hometransform)) (+ (* _normalizedtime 270.0) (.yaw (.rotation _hometransform)))) false false))
        (:`Finished`
          (`/Engine/EditorBlueprintResources/StandardMacros.FlipFlop`
            (:`A`
              (goto _label_2 :!via `ReverseFromEnd`))
            (:`B`
              (goto _label_2 :!via `PlayFromStart`))))))))

(event `self.Sphere.OnComponentBeginOverlap`
  (params (OverlappedComponent :type "PrimitiveComponent Object Reference") (OtherActor :type "Actor Object Reference") (OtherComp :type "PrimitiveComponent Object Reference") (OtherBodyIndex :type Integer) (bFromSweep :type Boolean) (SweepResult :type "HitResult Structure (by ref)"))
  (bind _asbp_player (cast `/Game/Blueprints/Character/BP_Player` OtherActor))
  (`GameplayStatics.PlaySoundAtLocation` "/Game/sOUND/crunchyBite.crunchyBite" (`self.K2_GetActorLocation`) (struct) 1.0 1.0 0.0 null null null null)
  (`/Game/Blueprints/Character/BP_Player.GetPowerUp` _asbp_player (`self.PowerType`))
  (`self.K2_DestroyActor`))

(fn `UserConstructionScript`)
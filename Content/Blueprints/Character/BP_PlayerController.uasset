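; Player controller that uses a camera actor from the level as the view and turns move and look input into four-way compass commands for BP_Player.
; On BeginPlay it blends the view to the CameraActor it finds.
; IA_Move and IA_Look map diagonal stick quadrants to north, east, south or west enum values, passed to PMove and PLook.
; Both axes must clear a small dead zone, so purely single-axis input triggers nothing.
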(event `self.ReceiveBeginPlay`
  (bind _returnvalue (`GameplayStatics.GetActorOfClass` "/Script/Engine.CameraActor"))
  (`self.SetViewTargetWithBlend` _returnvalue))

(event `EnhancedInput|/Game/ThirdPerson/Input/Actions/IA_Move`
  (params (ActionValue :type "Vector2D Structure") (ElapsedSeconds :type "Float (double-precision)") (TriggeredSeconds :type "Float (double-precision)") (InputAction :type "InputAction Object Reference" :default "/Game/ThirdPerson/Input/Actions/IA_Move.IA_Move"))
  (bind _returnvalue (> ActionValue_X 0.1))
  (bind _returnvalue_2 (> ActionValue_Y 0.1))
  (bind _returnvalue_3 (< ActionValue_Y -0.1))
  (bind _returnvalue_4 (< ActionValue_X -0.1))
  ;[1 1 1] MOMEMENT
  (:`Triggered`
    (`|ExecutionSequence`
      (:`then_0`
        (if (and _returnvalue _returnvalue_3)
          (bind _asbp_player (cast `/Game/Blueprints/Character/BP_Player` (`self.K2_GetPawn`)))
          (`/Game/Blueprints/Character/BP_Player.PMove` _asbp_player "NewEnumerator0")))
      (:`then_1`
        (if (and _returnvalue_2 _returnvalue)
          (bind _asbp_player_2 (cast `/Game/Blueprints/Character/BP_Player` (`self.K2_GetPawn`)))
          (`/Game/Blueprints/Character/BP_Player.PMove` _asbp_player_2 "NewEnumerator2")))
      (:`then_2`
        (if (and _returnvalue_4 _returnvalue_2)
          (bind _asbp_player_3 (cast `/Game/Blueprints/Character/BP_Player` (`self.K2_GetPawn`)))
          (`/Game/Blueprints/Character/BP_Player.PMove` _asbp_player_3 "NewEnumerator1")))
      (:`then_3`
        (if (and _returnvalue_4 _returnvalue_3)
          (bind _asbp_player_4 (cast `/Game/Blueprints/Character/BP_Player` (`self.K2_GetPawn`)))
          (`/Game/Blueprints/Character/BP_Player.PMove` _asbp_player_4 "NewEnumerator3"))))))

(event `EnhancedInput|/Game/ThirdPerson/Input/Actions/IA_Look`
  (params (ActionValue :type "Vector2D Structure") (ElapsedSeconds :type "Float (double-precision)") (TriggeredSeconds :type "Float (double-precision)") (InputAction :type "InputAction Object Reference" :default "/Game/ThirdPerson/Input/Actions/IA_Look.IA_Look"))
  (bind _returnvalue (> ActionValue_X 0.1))
  (bind _returnvalue_2 (> ActionValue_Y 0.1))
  (bind _returnvalue_3 (< ActionValue_Y -0.1))
  (bind _returnvalue_4 (< ActionValue_X -0.1))
  (:`Triggered`
    (`|ExecutionSequence`
      (:`then_0`
        (if (and _returnvalue _returnvalue_3)
          (bind _asbp_player (cast `/Game/Blueprints/Character/BP_Player` (`self.K2_GetPawn`)))
          (`/Game/Blueprints/Character/BP_Player.PLook` _asbp_player "NewEnumerator0")))
      (:`then_1`
        (if (and _returnvalue_2 _returnvalue)
          (bind _asbp_player_2 (cast `/Game/Blueprints/Character/BP_Player` (`self.K2_GetPawn`)))
          (`/Game/Blueprints/Character/BP_Player.PLook` _asbp_player_2 "NewEnumerator2")))
      (:`then_2`
        (if (and _returnvalue_4 _returnvalue_2)
          (bind _asbp_player_3 (cast `/Game/Blueprints/Character/BP_Player` (`self.K2_GetPawn`)))
          (`/Game/Blueprints/Character/BP_Player.PLook` _asbp_player_3 "NewEnumerator1")))
      (:`then_3`
        (if (and _returnvalue_4 _returnvalue_3)
          (bind _asbp_player_4 (cast `/Game/Blueprints/Character/BP_Player` (`self.K2_GetPawn`)))
          (`/Game/Blueprints/Character/BP_Player.PLook` _asbp_player_4 "NewEnumerator3"))))))

(fn `UserConstructionScript`)
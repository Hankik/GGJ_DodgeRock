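; Player character for a block-grid game that moves, turns, jumps, falls and swings to bat bricks or stun other players.
; Timelines drive motion in 100-unit cardinal steps, with line traces checking for blockers and ground.
; Flags queue inputs made mid-action, and FindNextMove chains into the queued action or a fall.
; Power-ups boost jump or swing or stun the player, while health calls forward to a damage component whose handlers only print.
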(event Custom|PMove
  (params (Direction :type E_MoveDirections%20Enum :default "NewEnumerator0"))
  ;[1 0.1458 0.3264] Player Move Logic
  (if (not (Variables|Default|GetisFalling))
    (if (Variables|PState|Getis%20Jumping)
      (Variables|Default|SethasMovedWhileJumping true)
      (elif (not (Variables|PState|GetisMoving))
        (Variables|PState|SetisMoving true)
        (bind _returnvalue (CallFunction|IsBlocked Direction))
        (if (not _returnvalue)
          (Variables|TempLoc|SetLocationAtMoveStart (Transformation|GetActorLocation))
          (switch Utilities|FlowControl|Switch|SwitchonE_MoveDirections Direction
            (:NewEnumerator0
              (Variables|PState|SetMoveDirection "(X=1.000000,Y=0.000000)")
              (bind _timenormalized (Timeline|MoveTimeline PlayFromStart)
                (:Update
                  (Transformation|SetActorLocation (Math|Vector|MakeVector (+ (* (.x (Variables|PState|GetMoveDirection)) 1e+02 _timenormalized) (.x (Variables|TempLoc|GetLocationAtMoveStart))) (+ (* (.y (Variables|PState|GetMoveDirection)) 1e+02 _timenormalized) (.y (Variables|TempLoc|GetLocationAtMoveStart))) (.z (Transformation|GetActorLocation))) false false))
                (:Finished
                  (Utilities|FlowControl|Delay 0.1)
                  (Variables|PState|SetisMoving false)
                  (CallFunction|FindNextMove))
                (:moveThunk
                  (Audio|PlaySoundatLocation "/Game/sOUND/moveThunk.moveThunk" (Transformation|GetActorLocation) "0, 0, 0" 0.7 1.0 0.0 0 0 0 0))))
            (:NewEnumerator1
              (Variables|PState|SetMoveDirection "(X=-1.000000,Y=0.000000)")
              (Timeline|MoveTimeline PlayFromStart))
            (:NewEnumerator2
              (Variables|PState|SetMoveDirection "(X=0.000000,Y=1.000000)")
              (Timeline|MoveTimeline PlayFromStart))
            (:NewEnumerator3
              (Variables|PState|SetMoveDirection "(X=0.000000,Y=-1.000000)")
              (Timeline|MoveTimeline PlayFromStart)))
          (else
            (CallFunction|FindNextMove)))))))

(event Custom|PLook
  (params (direction :type E_MoveDirections%20Enum :default "NewEnumerator0"))
  (bind _returnvalue (Transformation|GetActorLocation))
  ;[1 1 1] Player Rotate Orientation
  (Utilities|FlowControl|Sequence
    (:then_0
      (Variables|PState|SetLookDirCardinal direction)
      (if (Variables|PState|GetisMoving)
        (Variables|Default|SethasHoppedWhileMoving true)
        (else
          (Variables|Default|SetRotationAtLookStart (Transformation|GetActorRotation))
          (switch Utilities|FlowControl|Switch|SwitchonE_MoveDirections direction
            (:NewEnumerator0
              (Variables|Default|SetLookDirection 0.0)
              (bind _r (Timeline|Rotation%20Timeline PlayFromStart)
                (:Update
                  (Transformation|SetActorRotation (Math|Rotator|MakeRotator 0.0 0.0 (+ (* _r (- (Variables|Default|GetLookDirection) (.yaw (Variables|Default|GetRotationAtLookStart)))) (.yaw (Variables|Default|GetRotationAtLookStart))))))
                (:rotateBubble
                  (Audio|PlaySoundatLocation "/Game/sOUND/rotateBubble.rotateBubble" (Transformation|GetActorLocation) "0, 0, 0" 0.2 1.4 0.0 0 0 0 0))))
            (:NewEnumerator1
              (Variables|Default|SetLookDirection 1.8e+02)
              (Timeline|Rotation%20Timeline PlayFromStart))
            (:NewEnumerator2
              (Variables|Default|SetLookDirection 9e+01)
              (Timeline|Rotation%20Timeline PlayFromStart))
            (:NewEnumerator3
              (Variables|Default|SetLookDirection -9e+01)
              (Timeline|Rotation%20Timeline PlayFromStart))))))
    (:then_1
      (if (not (Variables|Default|GetisHopping))
        (Variables|Default|SetisHopping true)
        (Variables|Default|SetHeightAtStart (+ (.z _returnvalue) 0.0))
        (bind _height (Timeline|Jumping PlayFromStart)
          (:Update
            (Transformation|SetActorLocation (Math|Vector|MakeVector (.x _returnvalue) (.y _returnvalue) (+ (Variables|Default|GetHeightAtStart) (* _height 2e+01))) true true))
          (:Finished
            (Variables|Default|SetisHopping false)
            (CallFunction|FindNextMove)))))))

(event Custom|EndOfJumpMove
  ;[1 0.1458 0.3264] Player Move Logic
  (if (not (Variables|PState|GetisMoving))
    (Variables|PState|SetisMoving true)
    (bind _returnvalue (CallFunction|IsBlocked (stale Custom|PMove Direction)))
    (if (not _returnvalue)
      (Variables|TempLoc|SetLocationAtMoveStart (Transformation|GetActorLocation))
      (switch Utilities|FlowControl|Switch|SwitchonE_MoveDirections (stale Custom|PMove Direction)
        (:NewEnumerator0
          (Variables|PState|SetMoveDirection "(X=1.000000,Y=0.000000)")
          (bind _timenormalized (Timeline|MoveTimeline PlayFromStart)
            (:Update
              (Transformation|SetActorLocation (Math|Vector|MakeVector (+ (* (.x (Variables|PState|GetMoveDirection)) 1e+02 _timenormalized) (.x (Variables|TempLoc|GetLocationAtMoveStart))) (+ (* (.y (Variables|PState|GetMoveDirection)) 1e+02 _timenormalized) (.y (Variables|TempLoc|GetLocationAtMoveStart))) (.z (Transformation|GetActorLocation))) false false))
            (:Finished
              (Utilities|FlowControl|Delay 0.1)
              (Variables|PState|SetisMoving false)
              (CallFunction|FindNextMove))
            (:moveThunk
              (Audio|PlaySoundatLocation "/Game/sOUND/moveThunk.moveThunk" (Transformation|GetActorLocation) "0, 0, 0" 0.7 1.0 0.0 0 0 0 0))))
        (:NewEnumerator1
          (Variables|PState|SetMoveDirection "(X=-1.000000,Y=0.000000)")
          (Timeline|MoveTimeline PlayFromStart))
        (:NewEnumerator2
          (Variables|PState|SetMoveDirection "(X=0.000000,Y=1.000000)")
          (Timeline|MoveTimeline PlayFromStart))
        (:NewEnumerator3
          (Variables|PState|SetMoveDirection "(X=0.000000,Y=-1.000000)")
          (Timeline|MoveTimeline PlayFromStart)))
      (else
        (CallFunction|FindNextMove)))))

(event Custom|JumpAfterMoving
  (bind _returnvalue (Transformation|GetActorLocation))
  (if (not (Variables|PState|Getis%20Jumping))
    (if (not (Variables|Default|GetisFalling))
      (Variables|PState|Setis%20Jumping true)
      (CallFunction|ResetFallSound)
      (Variables|TempLoc|SetLocationAtJumpStart (Transformation|GetActorLocation))
      (bind _normalizedtime (Timeline|JumpTimeline PlayFromStart)
        (:Update
          (Transformation|SetActorLocation (Math|Vector|MakeVector (.x _returnvalue) (.y _returnvalue) (+ (.z (Variables|TempLoc|GetLocationAtJumpStart)) (* _normalizedtime 1e+02 (Variables|Default|GetJumpHeight)))) false false))
        (:Finished
          (Variables|PState|Setis%20Jumping false)
          (if (Variables|Default|GethasMovedWhileJumping)
            (Variables|Default|SethasMovedWhileJumping false)
            (CallFunction|EndOfJumpMove)
            (else
              (CallFunction|FindNextMove)))))
      (else
        (CallFunction|FindNextMove)))))

(event Custom|GetSlapped
  (bind _asbp_player_controller (Utilities|Casting|CastToBP_PlayerController (Pawn|GetController)))
  (Variables|/Game/Blueprints/Character/BP_PlayerController.BP_PlayerController_C|SetplayerStunned _asbp_player_controller true)
  (Utilities|FlowControl|Delay (Variables|Default|GetStunDuration))
  (Variables|/Game/Blueprints/Character/BP_PlayerController.BP_PlayerController_C|SetplayerStunned _asbp_player_controller false))

(event Custom|ResetFallSound
  (bind _returnvalue (Transformation|GetActorLocation))
  (bind _returnvalue_2 (- _returnvalue "0.000000,0.000000,50.000000"))
  (Utilities|FlowControl|DoOnce true) ; enters at Reset
)

(event Custom|GetPowerUp
  (params (Power :type E_PowerupTypes%20Enum :default "NewEnumerator0"))
  (switch Utilities|FlowControl|Switch|SwitchonE_PowerupTypes Power
    (:NewEnumerator0
      (Variables|Default|SetJumpHeight (+ (Variables|Default|GetJumpHeight) 1)))
    (:NewEnumerator2
      (Variables|Default|SetSwingPower (+ (Variables|Default|GetSwingPower) 1)))
    (:NewEnumerator3
      (bind _asbp_player_controller (Utilities|Casting|CastToBP_PlayerController (Pawn|GetController)))
      (Variables|/Game/Blueprints/Character/BP_PlayerController.BP_PlayerController_C|SetplayerStunned _asbp_player_controller true)
      (Utilities|FlowControl|Delay (Variables|Default|GetStunDuration))
      (Variables|/Game/Blueprints/Character/BP_PlayerController.BP_PlayerController_C|SetplayerStunned _asbp_player_controller false))))

(event Custom|Swing
  (bind _lookdircardinal (Variables|PState|GetLookDirCardinal))
  (if (not (Variables|Default|GetisSwinging))
    (Variables|Default|SetisSwinging true)
    (bind (_outhit _returnvalue) (CallFunction|IsBlocked _lookdircardinal))
    (if _returnvalue
      (bind _asbp_brick_base (Utilities|Casting|CastToBP_BrickBase (.HitActor (Collision|BreakHitResult _outhit)))
        (:then
          (Components|Timeline|SetPlayRate (Variables|/Game/Blueprints/Bricks/BP_BrickBase.BP_BrickBase_C|GetMoveTimeline _asbp_brick_base) (* 3.0 (Variables|Default|GetSwingPower)))
          (Default|Bat _asbp_brick_base _lookdircardinal)
          (Utilities|FlowControl|Delay 0.4 :!label _label))
        (:CastFailed
          (bind _asbp_player (Utilities|Casting|CastToBP_Player (.HitActor (Collision|BreakHitResult _outhit)))
            (:then
              (CallFunction|GetSlapped _asbp_player))
            (:CastFailed
              _))))
      (else
        (goto _label)))
    (Variables|Default|SetisSwinging false)))

(event Custom|Death
  (Development|PrintString "dead"))

(event Custom|Parried
  (Development|PrintString "parried"))

(event Custom|DamagerResponse
  (params (DamageResponse :type E_DamageResponse%20Enum :default "NewEnumerator0"))
  (Development|PrintString (Utilities|String|EnumtoString DamageResponse)))

(event Custom|PJump
  (bind _returnvalue (Transformation|GetActorLocation))
  (if (not (Variables|PState|GetisMoving))
    (if (not (Variables|PState|Getis%20Jumping))
      (if (not (Variables|Default|GetisFalling))
        (Variables|PState|Setis%20Jumping true)
        (CallFunction|ResetFallSound)
        (Variables|TempLoc|SetLocationAtJumpStart (Transformation|GetActorLocation))
        (bind _normalizedtime (Timeline|JumpTimeline PlayFromStart)
          (:Update
            (Transformation|SetActorLocation (Math|Vector|MakeVector (.x _returnvalue) (.y _returnvalue) (+ (.z (Variables|TempLoc|GetLocationAtJumpStart)) (* _normalizedtime 1e+02 (Variables|Default|GetJumpHeight)))) false false))
          (:Finished
            (Variables|PState|Setis%20Jumping false)
            (if (Variables|Default|GethasMovedWhileJumping)
              (Variables|Default|SethasMovedWhileJumping false)
              (CallFunction|EndOfJumpMove)
              (else
                (CallFunction|FindNextMove)))))
        (else
          (CallFunction|FindNextMove))))
    (else
      (Variables|Default|SethasJumpedWhileMoving true))))

(event Custom|PFall
  (bind _returnvalue (Transformation|GetActorLocation))
  (bind _returnvalue_2 (Transformation|GetActorLocation))
  (bind _returnvalue_3 (- _returnvalue "0.000000,0.000000,50.000000"))
  (Variables|Default|SetisFalling true)
  ;[1 1 1] Prevents snapping artifacts in fix alignment
  (Transformation|SetActorLocation (+ (Transformation|GetActorLocation) "0.000000,0.000000,10.000000") false false)
  (CallFunction|FixAlignment)
  (Variables|TempLoc|SetLocationAtFallStart (Transformation|GetActorLocation))
  (bind _normalizedtime (Timeline|FallTimeline PlayFromStart)
    (:Update
      (Transformation|SetActorLocation (Math|Vector|MakeVector (.x (Variables|TempLoc|GetLocationAtFallStart)) (.y (Variables|TempLoc|GetLocationAtFallStart)) (+ (.z (Variables|TempLoc|GetLocationAtFallStart)) (* _normalizedtime -1e+02))) false false)
      (bind (_outhit __) (CallFunction|FoundSomethingBelow 1.0))
      (if __
        (Transformation|SetActorLocation (Math|Vector|MakeVector (.x _returnvalue_2) (.y _returnvalue_2) (+ (Components|Capsule|GetScaledCapsuleHalfHeight (Variables|Collision|GetCapsuleComponent)) (.z (.Location (Collision|BreakHitResult _outhit))))) false false)
        (Audio|Components|Audio|Stop (Variables|Default|GetFallTimeline))
        (Utilities|FlowControl|DoOnce true
          (:Completed
            (Audio|PlaySoundatLocation "/Game/sOUND/footPat.footPat" _returnvalue_3 "0, 0, 0" 0.8 1.0 0.0 0 0 0 0)
            (Niagara|SpawnSystematLocation "/Game/VFX/poof.poof" _returnvalue_3)))))
    (:Finished
      (CallFunction|FindNextMove))))

(event Custom|FindNextMove
  (bind __ (CallFunction|FoundSomethingBelow 1e+01))
  (if __
    (Variables|PState|SetisMoving false)
    (Variables|Default|SetisFalling false)
    (Utilities|FlowControl|Sequence
      (:then_0
        (if (Variables|Default|GethasJumpedWhileMoving)
          (Variables|Default|SethasJumpedWhileMoving false)
          (CallFunction|JumpAfterMoving)
          (Transformation|SetActorLocation (+ (Transformation|GetActorLocation) "0.000000,0.000000,5.000000") false false :!label _label)
          (CallFunction|FixAlignment)))
      (:then_1
        (if (Variables|Default|GethasHoppedWhileMoving)
          (Variables|Default|SethasHoppedWhileMoving false)
          (CallFunction|PLook (Variables|PState|GetLookDirCardinal))
          (goto _label))))
    (else
      (CallFunction|PFall))))

(event Custom|FixAlignment
  (bind _returnvalue (Transformation|GetActorLocation))
  (Transformation|SetActorLocation (Math|Vector|MakeVector (* (/ (.x _returnvalue) 100) 1e+02) (* (/ (.y _returnvalue) 100) 1e+02) (* (/ (.z _returnvalue) 100) 1e+02)) false false))

(event EventBeginPlay
  (CallFunction|FindNextMove)
  (bind _asbp_player_controller (Utilities|Casting|CastToBP_PlayerController (Pawn|GetController)))
  (Input|AddMappingContext (PlayerController|LocalPlayerSubsystems|GetEnhancedInputLocalPlayerSubsystem _asbp_player_controller) "/Game/ThirdPerson/Input/IMC_Default.IMC_Default" 0 "(bIgnoreAllPressedKeysUntilRelease=True,bForceImmediately=False,bNotifyUserSettings=False)"))

(event Input|KeyboardEvents|DebugKeyQ
  (params (Key :type Key%20Structure :default "None") (ActionValue :type Input%20Action%20Value%20Structure))
  (:Pressed
    (switch Utilities|FlowControl|Switch|SwitchonE_MoveDirections (Variables|PState|GetLookDirCardinal)
      (:NewEnumerator0
        (CallFunction|PLook "NewEnumerator3"))
      (:NewEnumerator1
        (CallFunction|PLook "NewEnumerator2"))
      (:NewEnumerator2
        (CallFunction|PLook "NewEnumerator0"))
      (:NewEnumerator3
        (CallFunction|PLook "NewEnumerator1")))))

(fn ConstructionScript
  (bind _bpc_damagesystem (Variables|Default|GetBPC_DamageSystem))
  (EventDispatchers|BindEventtoOnDeath _bpc_damagesystem (EventDispatchers|CreateEvent :!event Custom|Death))
  (EventDispatchers|BindEventtoOnParried _bpc_damagesystem (EventDispatchers|CreateEvent :!event Custom|Parried))
  (EventDispatchers|BindEventtoOnDamageResponse _bpc_damagesystem (EventDispatchers|CreateEvent :!event Custom|DamagerResponse)))

(fn IsBlocked
  (params (Direction :type E_MoveDirections%20Enum :default "NewEnumerator0"))
  (bind _returnvalue (Transformation|GetActorLocation))
  (switch Utilities|FlowControl|Switch|SwitchonE_MoveDirections Direction
    (:NewEnumerator0
      (LocalVariables|SetCheckDirection "(X=1.000000,Y=0.000000)"))
    (:NewEnumerator1
      (LocalVariables|SetCheckDirection "(X=-1.000000,Y=0.000000)"))
    (:NewEnumerator2
      (LocalVariables|SetCheckDirection "(X=0.000000,Y=1.000000)"))
    (:NewEnumerator3
      (LocalVariables|SetCheckDirection "(X=0.000000,Y=-1.000000)")))
  (bind (_outhit _returnvalue_2) (Collision|LineTraceByChannel (Transformation|GetActorLocation) (Math|Vector|MakeVector (+ (.x _returnvalue) (* (.x (LocalVariables|GetCheckDirection)) 1e+02)) (+ (.y _returnvalue) (* (.y (LocalVariables|GetCheckDirection)) 1e+02)) (.z (Transformation|GetActorLocation))) "TraceTypeQuery3" false 0 "ForDuration"))
  (return _outhit _returnvalue_2))

(fn FoundSomethingBelow
  (params (HowFarBelow :type Float%20%28double-precision%29))
  (bind _returnvalue (Transformation|GetActorLocation))
  (bind _capsulecomponent (Variables|Collision|GetCapsuleComponent))
  (bind _capsulehalfheight (Variables|/Script/Engine.CapsuleComponent|GetCapsuleHalfHeight _capsulecomponent))
  (bind _returnvalue_2 (- _returnvalue (Math|Vector|MakeVector 0.0 0.0 _capsulehalfheight)))
  (bind (_outhit _returnvalue_3) (Collision|LineTraceByChannel _returnvalue_2 (+ _returnvalue_2 (* HowFarBelow (Math|Vector|VectorDown))) "TraceTypeQuery1" false 0 "ForDuration"))
  (return _outhit _returnvalue_3))

(fn GetCurrentHealth
  (return 0.0))

(fn GetMaxHealth
  (return (Variables|/Game/Blueprints/damageSystem/BPC_DamageSystem.BPC_DamageSystem_C|GetMaxHealth (Variables|Default|GetBPC_DamageSystem))))

(fn Heal
  (params (Amount :type Float%20%28double-precision%29))
  (bind _newhealth (Default|Heal (Variables|Default|GetBPC_DamageSystem) Amount))
  (return _newhealth))

(fn TakeDamage
  (params (damageInfo :type S%20Damage%20Info%20Structure))
  (bind _wasdamaged (Default|TakeDamage (Variables|Default|GetBPC_DamageSystem) damageInfo))
  (return _wasdamaged))
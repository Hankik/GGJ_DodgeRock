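; Game mode for a four-player local multiplayer, last-player-standing match.
; On BeginPlay it creates local players with controllers, then after a short delay numbers the player tag widgets by array order.
; It also initializes the WM input manager with the default mapping context and smart menu.
; Tick syncs the manager's player count and polls BP_Player actors, showing the win screen once when fewer than two remain.
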(event `self.ReceiveBeginPlay`
  (bind _returnvalue (`WM_ControllerFunctionLib.Get_WM_InputManager`))
  (`|ExecutionSequence`
    (:`then_1`
      (`GameplayStatics.CreatePlayer` 0)
      (`GameplayStatics.CreatePlayer` 1)
      (`GameplayStatics.CreatePlayer` 2)
      (`GameplayStatics.CreatePlayer` 3)
      (`KismetSystemLibrary.Delay` 0.2)
      (bind _foundwidgets (`WidgetBlueprintLibrary.GetAllWidgetsOfClass` "/Game/UI/W_PlayerTag.W_PlayerTag_C" false))
      (for (_array_element _array_index) _foundwidgets
        (set `/Game/UI/W_PlayerTag.Name` (`KismetStringLibrary.Concat_StrStr` "Player " (`KismetStringLibrary.Conv_IntToString` (+ _array_index 1))) _array_element)))
    (:`then_2`
      (`WM_InputManagerBase.setEnchancedInputContext` (`WM_ControllerFunctionLib.Get_WM_InputManager`) "/Game/ThirdPerson/Input/IMC_Default.IMC_Default")
      (bind _returnvalue_2 (`|CreateWidget` "/WM_InputManager_Plugin/WM_UMG/WM_InputManagerSmartMenu.WM_InputManagerSmartMenu_C"))
      (`UserWidget.AddToViewport` _returnvalue_2 0)
      (`WM_InputManagerBase.SetNumberOfPlayers` _returnvalue 4)
      (`WM_InputManager.BeginUMG` _returnvalue))))

(event `self.ReceiveTick`
  (params (DeltaSeconds :type "Float (single-precision)"))
  (bind _returnvalue (`self.GetNumPlayers`))
  (`WM_InputManagerBase.SetNumberOfPlayers` (`WM_ControllerFunctionLib.Get_WM_InputManager`) _returnvalue)
  (bind _outactors (`GameplayStatics.GetAllActorsOfClass` "/Game/Blueprints/Character/BP_Player.BP_Player_C"))
  (if (< (`KismetArrayLibrary.Array_Length` _outactors) 2)
    (`/Engine/EditorBlueprintResources/StandardMacros.DoOnce` false
      (:`Completed`
        (bind _returnvalue_2 (`|CreateWidget` "/Game/UI/UI_WinScreen.UI_WinScreen_C"))
        (`UserWidget.AddToViewport` _returnvalue_2 0)))))

(fn `UserConstructionScript`)
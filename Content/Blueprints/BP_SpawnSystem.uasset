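; BP_SpawnSystem spawns bricks of random types at random BP_BrickSpawnPoint actors in the level.
; On BeginPlay it gathers those spawn points and starts a looping timer at SpawnRate.
; Each tick of that timer spawns two bricks separated by a short random delay, then shrinks SpawnRate.
; The timer is never restarted, so the shrinking SpawnRate does not change its interval here.
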(event `self.ReceiveBeginPlay`
  (bind _outactors (`GameplayStatics.GetAllActorsOfClass` "/Game/Blueprints/Bricks/BP_BrickSpawnPoint.BP_BrickSpawnPoint_C"))
  (set `self.SpawnPoints` _outactors)
  (`KismetSystemLibrary.K2_SetTimerDelegate` (delegate `SpawnNewBrick`) (`self.SpawnRate`) true))

(event `SpawnNewBrick`
  (`self.SpawnB`)
  (`KismetSystemLibrary.Delay` (`KismetMathLibrary.RandomFloatInRange` 0.2 1.0))
  (`self.SpawnB`)
  (set `self.SpawnRate` (* (`self.SpawnRate`) 0.9)))

(event `SpawnB`
  (bind _bricktypes (`self.BrickTypes`))
  (bind _spawnpoints (`self.SpawnPoints`))
  (`/Game/Blueprints/Bricks/BP_BrickSpawnPoint.SpawnBrick` (`|GetArrayItem` _spawnpoints (`KismetMathLibrary.RandomInteger` (`KismetArrayLibrary.Array_Length` _spawnpoints))) (`|GetArrayItem` _bricktypes (`KismetMathLibrary.RandomInteger` (`KismetArrayLibrary.Array_Length` _bricktypes)))))

(fn `UserConstructionScript`)